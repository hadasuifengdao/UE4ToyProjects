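; Game mode for the runner game that detects when the player loses and triggers game over.
; Each tick, until the controller's GameEnd flag is set, it checks whether the runner character is dead or has been falling continuously for over two seconds.
; A long fall kills the character, and either case switches the menu to the game over widget and calls GameOver on the player controller.
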(event `self.ReceiveTick`
  (params (DeltaSeconds :type "Float (single-precision)"))
  (bind _asbp_runner_controller (cast `/Game/Runner/Blueprints/BP_RunnerController` (`GameplayStatics.GetPlayerController` 0)))
  (if (not (`RunnerController.gameEnd` _asbp_runner_controller))
    (bind _asbp_runner_character_1 (cast `/Game/Runner/Blueprints/BP_RunnerCharacter1` (`GameplayStatics.GetPlayerPawn` 0)))
    (if (`RunnerCharacter.BIsDie` _asbp_runner_character_1)
      (`self.ChangeMenuWidget` "/Game/UMG/UI_GameOver.UI_GameOver_C" :!label _label)
      (bind _asbp_runner_controller_2 (cast `/Game/Runner/Blueprints/BP_RunnerController` (`GameplayStatics.GetPlayerController` 0)))
      (`RunnerController.GameOver` _asbp_runner_controller_2)
      (elif (`NavMovementComponent.IsFalling` (`Character.CharacterMovement` _asbp_runner_character_1))
        (bind _output_get (set `self.FallTime` (+ (`self.FallTime`) DeltaSeconds)))
        (if (> _output_get 2.0)
          (`RunnerCharacter.Death` _asbp_runner_character_1)
          (goto _label))
        (else
          (set `self.FallTime` 0.0))))))

(fn `UserConstructionScript`)