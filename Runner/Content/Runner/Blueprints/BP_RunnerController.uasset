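; Runner controller that drives the magnet power-up, pulling nearby objects toward the player.
; While the living character's magnet flag is on, Tick spawns a particle effect and sphere-traces around the pawn.
; Blocking hits restart one shared timeline that lerps the hit actor to the player.
; A delay from the timeline update clears the character's flag and sets the controller's own, which blocks further pulls and is never reset here.
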(event `self.ReceiveTick`
  (params (DeltaSeconds :type "Float (single-precision)"))
  (bind _returnvalue (`self.K2_GetActorLocation` (`GameplayStatics.GetPlayerPawn` 0)))
  (if (not (`self.UseMagnet`))
    (bind _asbp_runner_character_1 (cast `/Game/Runner/Blueprints/BP_RunnerCharacter1` (`GameplayStatics.GetPlayerPawn` 0)))
    (if (`RunnerCharacter.BIsDie` _asbp_runner_character_1)
      _
      (elif (`RunnerCharacter.UseMagnet` _asbp_runner_character_1)
        (`GameplayStatics.SpawnEmitterAtLocation` "/Game/Effects/ParticleSystems/Weapons/AssaultRifle/Muzzle/P_AssaultRifle_MF.P_AssaultRifle_MF" _returnvalue)
        (bind _outhits (`KismetSystemLibrary.SphereTraceMultiForObjects` _returnvalue (+ _returnvalue (0.0 0.0 15.0)) 1000.0 (`self.NewVar_0`)))
        (for _array_element _outhits
          (bind (_bblockinghit _binitialoverlap _time _location _impactpoint _normal _impactnormal _physmat _hitactor) (`GameplayStatics.BreakHitResult` _array_element))
          (if _bblockinghit
            (bind (_direction _alpha) (`Timeline|Timeline_0` :!via `PlayFromStart`)
              (:`Update`
                (`self.K2_SetActorLocation` _hitactor (`KismetMathLibrary.VLerp` (`self.K2_GetActorLocation` _hitactor) (`self.K2_GetActorLocation` (`GameplayStatics.GetPlayerPawn` 0)) _alpha) false false)
                (`KismetSystemLibrary.Delay` 10.0)
                (bind _asbp_runner_character_1_2 (cast `/Game/Runner/Blueprints/BP_RunnerCharacter1` (`GameplayStatics.GetPlayerPawn` 0)))
                (set `RunnerCharacter.UseMagnet` false _asbp_runner_character_1_2)
                (set `self.UseMagnet` true)))))))))

(fn `UserConstructionScript`)