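; BP_FloorTile_Jump is a floor tile for a runner game, named as a jump variant.
; On BeginPlay it adds a child actor component at AttachPoint1's relative transform.
; When BP_RunnerCharacter1 overlaps EndTrigger, it searches its child actors, including descendants, for BP_Skid and sets that skid's Floor to a fixed scale and relative location.
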(event `self.ReceiveBeginPlay`
  (`AddComponent|NODE_AddChildActorComponent-0` :`RelativeTransform` (`SceneComponent.GetRelativeTransform` (`self.AttachPoint1`))))

(event `self.EndTrigger.OnComponentBeginOverlap`
  (params (OverlappedComponent :type "PrimitiveComponent Object Reference") (OtherActor :type "Actor Object Reference") (OtherComp :type "PrimitiveComponent Object Reference") (OtherBodyIndex :type Integer) (bFromSweep :type Boolean) (SweepResult :type "HitResult Structure (by ref)"))
  (cast `/Game/Runner/Blueprints/BP_RunnerCharacter1` OtherActor)
  (for _array_element (`self.GetAllChildActors` true)
    (bind _asbp_skid (cast `/Game/Item/BP_Skid` _array_element))
    (bind _floor (`Skid.Floor` _asbp_skid))
    (`SceneComponent.SetRelativeScale3D` _floor (7.0 10.0 0.1))
    (`SceneComponent.K2_SetRelativeLocation` _floor (350.0 0.0 0.0) false false)))

(fn `UserConstructionScript`)