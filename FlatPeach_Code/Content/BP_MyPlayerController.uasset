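; Player controller that updates tile occupancy for planting and shovel actions on Cube actors.
; Tick polls two flags: BPlant marks a Cube as Occupied, BUseShovel clears one, and each flag resets afterward.
; The target is picked by using the index from Change or ChangeShovels, neither defined in this graph, into a fresh GetAllActorsOfClass list, so it depends on that list's order.
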(event `self.ReceiveBeginPlay`)

(event `self.ReceiveTick`
  (params (DeltaSeconds :type "Float (single-precision)"))
  (if (`self.BPlant`)
    (bind _returnvalue (`self.Change`))
    (bind _outactors (`GameplayStatics.GetAllActorsOfClass` "/Script/FlatPeach.Cube"))
    (set `Cube.Occupied` true (`|GetArrayItem` _outactors _returnvalue))
    (set `self.BPlant` false))
  (if (`self.BUseShovel`)
    (bind _returnvalue_2 (`self.ChangeShovels`))
    (bind _outactors_2 (`GameplayStatics.GetAllActorsOfClass` "/Script/FlatPeach.Cube"))
    (set `Cube.Occupied` false (`|GetArrayItem` _outactors_2 _returnvalue_2))
    (set `self.BUseShovel` false)))

(fn `UserConstructionScript`)