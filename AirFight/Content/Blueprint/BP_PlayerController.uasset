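; Player controller for a round-based multiplayer game that handles the local camera and the round-flow UI.
; After a short delay on BeginPlay, the local controller yaws the MainCamera-tagged actor to its own facing and sets it as view target.
; Client events show cached waiting, countdown and result widgets, switching HUD visibility, cursor and input mode.
; A server event reports restart readiness to BP_GameMode.
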(event `self.ReceiveBeginPlay`
  ;[1 1 1] Set the orientation of the main camera
  (`KismetSystemLibrary.Delay` 0.5)
  (if (`self.IsLocalPlayerController` self)
    (bind _outactors (`GameplayStatics.GetAllActorsWithTag` "MainCamera"))
    (bind _output (`|GetArrayItem` _outactors))
    (`self.K2_SetActorRotation` _output (`KismetMathLibrary.MakeRotator` (.roll (`self.K2_GetActorRotation` _output)) (.pitch (`self.K2_GetActorRotation` _output)) (.yaw (`self.K2_GetActorRotation`))) false)
    (`self.SetViewTargetWithBlend` _output)))

(event `ShowWaitForAnPlayer`
  ;[1 1 1] Show wait for an player
  (`/Engine/EditorBlueprintResources/StandardMacros.IsValid` (`self.Waitforanplayer`)
    (:`Is Valid`
      _)
    (:`Is Not Valid`
      (bind _returnvalue (`|CreateWidget` "/Game/UI/UI_Waitforanplayer.UI_Waitforanplayer_C" self))
      (set `self.Waitforanplayer` _returnvalue)))
  (`UserWidget.AddToViewport` (`self.Waitforanplayer`) 0))

(event `Client_ShowRoundStartCountDownWidget`
  (bind _waitforanplayer (`self.Waitforanplayer`))
  ;[1 1 1] Show CountDown
  (`/Engine/EditorBlueprintResources/StandardMacros.IsValid` (`self.RoundStartCountDownWidget`)
    (:`Is Valid`
      _)
    (:`Is Not Valid`
      (bind _returnvalue (`|CreateWidget` "/Game/UI/UI_RoundStartCountDown.UI_RoundStartCountDown_C" self))
      (set `self.RoundStartCountDownWidget` _returnvalue)))
  (`UserWidget.AddToViewport` (`self.RoundStartCountDownWidget`) 0)
  (`/Engine/EditorBlueprintResources/StandardMacros.IsValid` _waitforanplayer
    (:`Is Valid`
      (if (`Widget.IsInViewport` _waitforanplayer)
        (`Widget.RemoveFromParent` _waitforanplayer)
        (set `self.bShowMouseCursor` false)
        (`WidgetBlueprintLibrary.SetInputMode_UIOnlyEx` self)
        (bind _asbp_game_hud (cast `/Game/Blueprint/BP_GameHUD` (`self.GetHUD`)))
        (`/Game/Blueprint/BP_GameHUD.ToggleAllElementsVisibility` _asbp_game_hud false)))))

(event `Client_OnCountDownEnd`
  ;[1 1 1] CoundDown is End before starting a new round
  (bind _asbp_game_hud (cast `/Game/Blueprint/BP_GameHUD` (`self.GetHUD`)))
  (`/Game/Blueprint/BP_GameHUD.ToggleAllElementsVisibility` _asbp_game_hud true)
  (set `self.bShowMouseCursor` false)
  (`WidgetBlueprintLibrary.SetInputMode_GameOnly` self))

(event `Client_ShowRoundResult`
  (params (RoundResult :type String))
  ;[1 1 1] Show Round Result
  (`KismetSystemLibrary.Delay` 1.0)
  (`/Engine/EditorBlueprintResources/StandardMacros.IsValid` (`self.RoundResultWidget`)
    (:`Is Valid`
      _)
    (:`Is Not Valid`
      (bind _returnvalue (`|CreateWidget` "/Game/UI/UI_RoundResult.UI_RoundResult_C" self))
      (bind _output_get (set `self.RoundResultWidget` _returnvalue))))
  (`UserWidget.AddToViewport` _output_get 0)
  (`/Game/UI/UI_RoundResult.SetRoundResult` _output_get RoundResult)
  (set `self.bShowMouseCursor` true)
  (`WidgetBlueprintLibrary.SetInputMode_UIOnlyEx` self)
  (bind _asbp_game_hud (cast `/Game/Blueprint/BP_GameHUD` (`self.GetHUD`)))
  (`/Game/Blueprint/BP_GameHUD.ToggleAllElementsVisibility` _asbp_game_hud false))

(event `Server_AttemptToRestartRound`
  ;[1 1 1] Tell server this player is ready to restart round
  (bind _asbp_game_mode (cast `/Game/Blueprint/BP_GameMode` (`GameplayStatics.GetGameMode`)))
  (`/Game/Blueprint/BP_GameMode.OnPlayerReadyToRestartRound` _asbp_game_mode self))

(fn `UserConstructionScript`)