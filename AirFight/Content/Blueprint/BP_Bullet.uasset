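; BP_Bullet is a networked projectile that flies forward at MoveSpeed, damages player pawns on impact and explodes.
; Tick moves it with a swept world offset through Client_Move, called directly on authority and routed via Server_Move on remotes.
; On a Box hit, authority applies damage to any BP_PlayerPawn and calls a client event that hides the bullet and plays explosion particles and sound.
; Authority then disables collision and destroys the actor after a short delay.
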(event `self.ReceiveTick`
  (params (DeltaSeconds :type "Float (single-precision)"))
  (`/Engine/EditorBlueprintResources/ActorMacros.Switch Has Authority`
    (:`Authority`
      (`self.Client_Move` DeltaSeconds))
    (:`Remote`
      (`self.Server_Move` DeltaSeconds))))

(event `Server_Move`
  (params (InDeltaTime :type "Float (double-precision)"))
  (`self.Client_Move` InDeltaTime))

(event `Client_Move`
  (params (InDeltaTime :type "Float (double-precision)"))
  (`self.K2_AddActorWorldOffset` (* (`self.GetActorForwardVector`) (* InDeltaTime (`self.MoveSpeed`))) true))

(event `self.Box.OnComponentHit`
  (params (HitComponent :type "PrimitiveComponent Object Reference") (OtherActor :type "Actor Object Reference") (OtherComp :type "PrimitiveComponent Object Reference") (NormalImpulse :type "Vector Structure") (Hit :type "HitResult Structure (by ref)"))
  (bind (_bblockinghit _binitialoverlap _time _location _impactpoint _normal _impactnormal _physmat _hitactor) (`GameplayStatics.BreakHitResult` Hit))
  (`/Engine/EditorBlueprintResources/ActorMacros.Switch Has Authority`
    (:`Authority`
      (bind _asbp_player_pawn (cast `/Game/Blueprint/BP_PlayerPawn` _hitactor)
        (:`then`
          (`GameplayStatics.ApplyDamage` _asbp_player_pawn (`self.Damage`) null self))
        (:`CastFailed`
          _))
      (`self.Client_PlayBulletExplosionEffect` _location)
      (`PrimitiveComponent.SetCollisionEnabled` (`self.Box`) "NoCollision")
      (`KismetSystemLibrary.Delay` 0.2)
      (`self.K2_DestroyActor`))))

(event `Client_PlayBulletExplosionEffect`
  (params (Location :type "Vector Structure"))
  (`self.SetActorHiddenInGame` true)
  (`GameplayStatics.SpawnEmitterAtLocation` "/Game/Particles/P_Pixel_Explosion.P_Pixel_Explosion" Location)
  (`GameplayStatics.PlaySoundAtLocation` "/Game/Audio/A_Explosion.A_Explosion" Location))

(fn `UserConstructionScript`)