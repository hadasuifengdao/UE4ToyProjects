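; Networked player pawn with an engine trail that glides forward to a start point, then takes sideways movement and fire input.
; Strafe speed is interpolated and banks the model, while local and remote pawns get different materials.
; A looping timer rate-limits held fire, with server events spawning bullets and client events playing effects.
; Damage lowers PlayerState HP; at zero the pawn unpossesses, explodes, is destroyed and tells the GameMode to end the round.
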(event `self.ReceiveBeginPlay`
  (bind _returnvalue (`self.GetActorForwardVector`))
  (bind _staticmesh (`self.StaticMesh`))
  (set `self.DisiredLocation` (+ (`self.K2_GetActorLocation`) (* _returnvalue 150.0)))
  (`ParticleSystemComponent.SetVectorParameter` (`self.P_EngineTrail`) "Direction" (`KismetMathLibrary.MakeVector` 0.0 0.0 (* (.x _returnvalue) -200.0)))
  (`KismetSystemLibrary.Delay` 0.5)
  (if (`self.IsLocallyControlled`)
    (`PrimitiveComponent.SetMaterial` _staticmesh 0 "/Engine/MapTemplates/Materials/BasicAsset01.BasicAsset01")
    (else
      (`PrimitiveComponent.SetMaterial` _staticmesh 0 "/Engine/MapTemplates/Materials/BasicAsset03.BasicAsset03"))))

(event `self.ReceiveTick`
  (params (DeltaSeconds :type "Float (single-precision)"))
  (bind _scene (`self.Scene`))
  (bind _returnvalue (`KismetMathLibrary.VSize` (- (`self.DisiredLocation`) (`self.K2_GetActorLocation`))))
  (if (`self.IsInputEnabled`)
    (bind _returndirection (`self.Movement` (`self.HozSpeed`) (`self.HozMoveDirection`) DeltaSeconds))
    (bind _output_get (set `self.HozSpeed` _returndirection))
    (`self.K2_AddActorWorldOffset` (* (`self.GetActorRightVector`) _output_get) true)
    (`SceneComponent.K2_SetRelativeRotation` _scene (`KismetMathLibrary.RInterpTo_Constant` (`SceneComponent.RelativeRotation` _scene) (`KismetMathLibrary.MakeRotator` (* (`self.HozSpeed`) 20.0)) DeltaSeconds 40.0) false false)
    (else
      (`self.K2_AddActorWorldOffset` (* (* (`self.GetActorForwardVector`) DeltaSeconds) (`self.Speed`)) true)
      (if (or (<= _returnvalue 1.0) (>= _returnvalue 155.0))
        (set `self.IsInputEnabled` true)
        (`self.K2_SetActorLocation` (`self.DisiredLocation`) false true)))))

(event `InputAxis|MoveRight`
  (params (AxisValue :type "Float (single-precision)"))
  (`self.Server_UpdateMoveRightInputAxisValue` AxisValue)
  (set `self.HozMoveDirection` AxisValue))

(event `Server_UpdateMoveRightInputAxisValue`
  (params (HozMoveDirection :type "Float (double-precision)"))
  (set `self.HozMoveDirection` HozMoveDirection))

(event `InputAction|Fire`
  (params (Key :type "Key Structure" :default "AnyKey"))
  (:`Pressed`
    (if (`self.IsInputEnabled`)
      (set `self.IsFireActionActivated` true)
      (if (`self.CanFire`)
        (`self.ServerFire`)
        (set `self.CanFire` false)
        (bind _returnvalue (`KismetSystemLibrary.K2_SetTimerDelegate` (delegate `ContinousFire`) 0.5 true))
        (set `self.FireTimerHandle` _returnvalue))))
  (:`Released`
    (set `self.IsFireActionActivated` false)))

(event `ContinousFire`
  (set `self.CanFire` true)
  (if (`self.IsFireActionActivated`)
    (`self.ServerFire`)
    (set `self.CanFire` false)
    (else
      (`KismetSystemLibrary.K2_ClearAndInvalidateTimerHandle` (`self.FireTimerHandle`)))))

(event `ServerFire`
  (bind _returnvalue (`SceneComponent.K2_GetComponentLocation` (`self.BulletSpawnPosition`)))
  (`|SpawnActorFromClass` "/Game/Blueprint/BP_Bullet.BP_Bullet_C" (`KismetMathLibrary.MakeTransform` _returnvalue (`self.K2_GetActorRotation`)) "Undefined" "OverrideRootScale" null null)
  (`self.ClientPlayFireSound` _returnvalue))

(event `ClientPlayFireSound`
  (params (Location :type "Vector Structure"))
  (`GameplayStatics.PlaySoundAtLocation` "/Game/Audio/A_Shot.A_Shot" Location))

(event `self.ReceiveAnyDamage`
  (params (Damage :type "Float (single-precision)") (DamageType :type "DamageType Object Reference") (InstigatedBy :type "Controller Object Reference") (DamageCauser :type "Actor Object Reference"))
  (bind _asbp_player_state (cast `/Game/Blueprint/BP_PlayerState` (`self.PlayerState`)))
  (bind _returnvalue (- (`/Game/Blueprint/BP_PlayerState.CurrentHP` _asbp_player_state) (`KismetMathLibrary.FTrunc` Damage)))
  (if (> _returnvalue 0)
    (set `/Game/Blueprint/BP_PlayerState.CurrentHP` _returnvalue _asbp_player_state)
    (else
      (set `/Game/Blueprint/BP_PlayerState.CurrentHP` 0 _asbp_player_state)
      (`Controller.UnPossess` (`self.GetController`))
      (`PrimitiveComponent.SetCollisionEnabled` (`self.Box`) "NoCollision")
      (`self.Client_OnKilled`)
      (`KismetSystemLibrary.Delay` 0.2)
      (`self.K2_DestroyActor`)
      (bind _asbp_game_mode (cast `/Game/Blueprint/BP_GameMode` (`GameplayStatics.GetGameMode`)))
      (`/Game/Blueprint/BP_GameMode.EndRound` _asbp_game_mode))))

(event `Client_OnKilled`
  (bind _returnvalue (`self.K2_GetActorLocation`))
  (`self.SetActorHiddenInGame` true)
  (`GameplayStatics.SpawnEmitterAtLocation` "/Game/Particles/P_Pixel_Explosion_Player.P_Pixel_Explosion_Player" _returnvalue)
  (`GameplayStatics.SpawnSoundAtLocation` "/Game/Audio/A_Explosion.A_Explosion" _returnvalue))

(fn `Movement`
  (params (Speed :type "Float (double-precision)") (Direction :type "Float (double-precision)") (DeltaTime :type "Float (double-precision)"))
  (returns (ReturnDirection :type "Float (double-precision)"))
  (return (`KismetMathLibrary.FInterpTo` Speed (* Direction (`self.SpeedToDirectionFactor`)) DeltaTime 4.0)))

(fn `UserConstructionScript`)