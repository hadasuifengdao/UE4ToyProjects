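; BP_GameHUD is a HUD Blueprint that shows or hides the game's UI_HUD widget for its owning player.
; ToggleAllElementsVisibility lazily creates and caches the widget on first show, then adds it to the viewport.
; Hiding removes the widget from its parent only if it is valid and in the viewport, keeping the cached instance for later.
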(fn `ToggleAllElementsVisibility`
  (params (InToggleFlag :type Boolean))
  (bind _ui_hudwidget (`self.UI_HUDWidget`))
  (if InToggleFlag
    (`/Engine/EditorBlueprintResources/StandardMacros.IsValid` (`self.UI_HUDWidget`)
      (:`Is Valid`
        _)
      (:`Is Not Valid`
        (bind _returnvalue (`|CreateWidget` "/Game/UI/UI_HUD.UI_HUD_C" (`self.GetOwningPlayerController`)))
        (set `self.UI_HUDWidget` _returnvalue)))
    (`UserWidget.AddToViewport` (`self.UI_HUDWidget`) 0)
    (else
      (`/Engine/EditorBlueprintResources/StandardMacros.IsValid` _ui_hudwidget
        (:`Is Valid`
          (if (`Widget.IsInViewport` _ui_hudwidget)
            (`Widget.RemoveFromParent` _ui_hudwidget)))))))

(fn `UserConstructionScript`)