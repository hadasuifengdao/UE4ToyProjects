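; Game mode that runs a round-based two-player duel, from login to round result.
; Login registers controllers and marks the first as host; restarts, triggered by a Tick-polled flag or both players readying, respawn pawns at index-tagged PlayerStarts and show countdowns.
; EndRound, guarded against re-entry, waits briefly, compares HP to send win, lose or draw results and score the winner, then clears ready flags and destroys pawns.
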(event `self.ReceiveTick`
  (params (DeltaSeconds :type "Float (single-precision)"))
  ;[1 1 1] 检测是否开始游戏
  (if (`self.IsRoundStart`)
    (`self.Restart Round`)
    (set `self.IsRoundStart` false)))

(event `self.K2_PostLogin`
  (params (NewPlayer :type "PlayerController Object Reference"))
  (bind _playerlist (`self.Playerlist`))
  ;[1 1 1] Login
  (bind _asbp_player_controller (cast `/Game/Blueprint/BP_PlayerController` NewPlayer))
  (`KismetArrayLibrary.Array_AddUnique` _playerlist _asbp_player_controller)
  (if (== (`KismetArrayLibrary.Array_Length` _playerlist) 1)
    (bind _playerstate (`Controller.PlayerState` _asbp_player_controller))
    (bind _asbp_player_state (cast `/Game/Blueprint/BP_PlayerState` _playerstate))
    (set `/Game/Blueprint/BP_PlayerState.IsHoster` true _asbp_player_state)
    (else
      (bind _asbp_player_state_2 (cast `/Game/Blueprint/BP_PlayerState` _playerstate))
      (set `/Game/Blueprint/BP_PlayerState.IsHoster` false _asbp_player_state_2)))
  (`/Game/Blueprint/BP_PlayerController.ShowWaitForAnPlayer` _asbp_player_controller))

(event `Restart Round`
  ;[1 1 1] Restart Round
  (set `self.IsRoundEnd` false)
  (for _array_element (`self.Playerlist`)
    (`self.ResetPlayer` _array_element)
    (`/Game/Blueprint/BP_PlayerController.Client_ShowRoundStartCountDownWidget` _array_element)))

(event `ResetPlayer`
  (params (InPlayer :type "/Game/Blueprint/BP_PlayerController Object Reference"))
  (bind _returnvalue (`Controller.K2_GetPawn` InPlayer))
  ;[1 1 1] Destroy the origin pawn and spawn a new one at a desired PlayerStart
  (bind _asbp_player_state (cast `/Game/Blueprint/BP_PlayerState` (`Controller.PlayerState` InPlayer)))
  (set `/Game/Blueprint/BP_PlayerState.IsReady` false _asbp_player_state)
  (set `/Game/Blueprint/BP_PlayerState.CurrentHP` 100 _asbp_player_state)
  (`/Engine/EditorBlueprintResources/StandardMacros.IsValid` _returnvalue
    (:`Is Valid`
      (`self.K2_DestroyActor` _returnvalue))
    (:`Is Not Valid`
      _))
  (bind _outactors (`GameplayStatics.GetAllActorsWithTag` (`KismetStringLibrary.Conv_StringToName` (`KismetStringLibrary.Concat_StrStr` "PlayerStart_" (`KismetStringLibrary.Conv_IntToString` (`KismetArrayLibrary.Array_Find` (`self.Playerlist`) InPlayer))))))
  (bind _returnvalue_2 (`|SpawnActorFromClass` "/Game/Blueprint/BP_PlayerPawn.BP_PlayerPawn_C" (`self.GetTransform` (`|GetArrayItem` _outactors)) "Undefined" "OverrideRootScale" null null))
  (`Controller.Possess` InPlayer _returnvalue_2))

(event `EndRound`
  ;[1 1 1] The round will be over if one of the player is killed
  (if (not (`self.IsRoundEnd`))
    (set `self.IsRoundEnd` true)
    (`KismetSystemLibrary.Delay` 1.0)
    (`self.RoundResultCheck`)
    (for _array_element (`self.Playerlist`)
      (bind _asbp_player_state (cast `/Game/Blueprint/BP_PlayerState` (`Controller.PlayerState` _array_element)))
      (set `/Game/Blueprint/BP_PlayerState.IsReady` false _asbp_player_state)
      (bind _returnvalue (`Controller.K2_GetPawn` _array_element))
      (`/Engine/EditorBlueprintResources/StandardMacros.IsValid` _returnvalue
        (:`Is Valid`
          (`self.K2_DestroyActor` _returnvalue))))))

(event `OnPlayerReadyToRestartRound`
  (params (InPlayer :type "/Game/Blueprint/BP_PlayerController Object Reference"))
  ;[1 1 1] Check whether if both players are ready to restart round
  (bind _asbp_player_state (cast `/Game/Blueprint/BP_PlayerState` (`Controller.PlayerState` InPlayer)))
  (set `/Game/Blueprint/BP_PlayerState.IsReady` true _asbp_player_state)
  (for _array_element (`self.Playerlist`)
    (if (!= InPlayer _array_element)
      (bind _asbp_player_state_2 (cast `/Game/Blueprint/BP_PlayerState` (`Controller.PlayerState` _array_element)))
      (if (`/Game/Blueprint/BP_PlayerState.IsReady` _asbp_player_state_2)
        (`self.Restart Round`)
        (else
          (`/Game/Blueprint/BP_PlayerController.ShowWaitForAnPlayer` InPlayer))))))

(fn `DispatchLoseAndWinRoundResult`
  (params (InWinner :type "/Game/Blueprint/BP_PlayerController Object Reference") (InLoser :type "/Game/Blueprint/BP_PlayerController Object Reference"))
  (`/Game/Blueprint/BP_PlayerController.Client_ShowRoundResult` InWinner "Win!")
  (bind _asbp_player_state (cast `/Game/Blueprint/BP_PlayerState` (`Controller.PlayerState` InWinner)))
  (`/Game/Blueprint/BP_PlayerState.IncreasePlayerScore` _asbp_player_state)
  (`/Game/Blueprint/BP_PlayerController.Client_ShowRoundResult` InLoser "Lose!"))

(fn `RoundResultCheck`
  (locals (Player1StateRef :type "/Game/Blueprint/BP_PlayerState Object Reference") (Player2StateRef :type "/Game/Blueprint/BP_PlayerState Object Reference"))
  (bind _playerlist (`self.Playerlist`))
  (bind _playerlist_2 (`self.Playerlist`))
  (bind _asbp_player_state (cast `/Game/Blueprint/BP_PlayerState` (`Controller.PlayerState` (`|GetArrayItem` (`self.Playerlist`)))))
  (set `local.Player1StateRef` _asbp_player_state)
  (bind _asbp_player_state_2 (cast `/Game/Blueprint/BP_PlayerState` (`Controller.PlayerState` (`|GetArrayItem` (`self.Playerlist`) 1))))
  (set `local.Player2StateRef` _asbp_player_state_2)
  (if (and (== (`/Game/Blueprint/BP_PlayerState.CurrentHP` (`local.Player1StateRef`)) 0) (== (`/Game/Blueprint/BP_PlayerState.CurrentHP` (`local.Player2StateRef`)) 0))
    (for _array_element (`self.Playerlist`)
      (`/Game/Blueprint/BP_PlayerController.Client_ShowRoundResult` _array_element "平局"))
    (elif (!= (`/Game/Blueprint/BP_PlayerState.CurrentHP` (`local.Player1StateRef`)) 0)
      (`self.DispatchLoseAndWinRoundResult` (`|GetArrayItem` _playerlist) (`|GetArrayItem` _playerlist 1))
      (else
        (`self.DispatchLoseAndWinRoundResult` (`|GetArrayItem` _playerlist_2 1) (`|GetArrayItem` _playerlist_2))))))

(fn `UserConstructionScript`)